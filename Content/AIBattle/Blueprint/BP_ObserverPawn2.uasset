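; Observer pawn in AIBattle that gives a bird's-eye camera with panning and zoom, starting at maximum height above the world origin.
; Axis inputs move the actor directly within clamped bounds, with zoom changing its Z height.
; When input stops, the last axis value decays each tick for a gliding stop, without delta-time scaling.
; During zoom, PitchCurve maps camera height to a pitch offset from straight down.
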(event `InputAxis|Zoom`
  (params (AxisValue :type "Float (single-precision)"))
  (bind (_returnvalue_x _returnvalue_y _returnvalue_z) (`KismetMathLibrary.BreakVector` (`self.K2_GetActorLocation`)))
  (bind (_returnvalue_x_2 _returnvalue_y_2 _returnvalue_z_2) (`KismetMathLibrary.BreakVector` (`self.K2_GetActorLocation`)))
  (bind (_returnvalue_x_3 _returnvalue_y_3 _returnvalue_z_3) (`KismetMathLibrary.BreakVector` (`SceneComponent.K2_GetComponentLocation` (`self.Camera`))))
  ;[1 1 1] ZoomIn
  (if (== AxisValue 0.0)
    (if (not (== (`self.LastZoomingValue`) 0.0))
      (`self.K2_SetActorLocation` (`KismetMathLibrary.MakeVector` _returnvalue_x_2 _returnvalue_y_2 (`KismetMathLibrary.FClamp` (+ (* (`self.LastZoomingValue`) 100.0) _returnvalue_z_2) 750.0 13500.0)))
      (set `self.LastZoomingValue` (`KismetMathLibrary.FClamp` (* (`self.LastZoomingValue`) 0.91) -1.0 1.0))
      (`self.K2_SetActorRotation` (`KismetMathLibrary.MakeRotator` 0.0 (+ (`CurveFloat.GetFloatValue` (`self.PitchCurve`) _returnvalue_z_3) -90.0)) :!label _label))
    (else
      (set `self.LastZoomingValue` AxisValue)
      (`self.K2_SetActorLocation` (`KismetMathLibrary.MakeVector` _returnvalue_x _returnvalue_y (`KismetMathLibrary.FClamp` (+ (* AxisValue 100.0) _returnvalue_z) 750.0 13500.0)))
      (goto _label))))

(event `InputAxis|MoveForward`
  (params (AxisValue :type "Float (single-precision)"))
  (bind (_returnvalue_x _returnvalue_y _returnvalue_z) (`KismetMathLibrary.BreakVector` (`self.K2_GetActorLocation`)))
  (bind (_returnvalue_x_2 _returnvalue_y_2 _returnvalue_z_2) (`KismetMathLibrary.BreakVector` (`self.K2_GetActorLocation`)))
  ;[1 1 1] MoveForward
  (if (== AxisValue 0.0)
    (if (not (== (`self.LastMoveFwdValue`) 0.0))
      (`self.K2_SetActorLocation` (`KismetMathLibrary.MakeVector` (`KismetMathLibrary.FClamp` (+ (* (`self.LastMoveFwdValue`) 30.0) _returnvalue_x_2) -7500.0 4900.0) _returnvalue_y_2 _returnvalue_z_2))
      (set `self.LastMoveFwdValue` (`KismetMathLibrary.FClamp` (* (`self.LastMoveFwdValue`) 0.95) -1.0)))
    (else
      (set `self.LastMoveFwdValue` AxisValue)
      (`self.K2_SetActorLocation` (`KismetMathLibrary.MakeVector` (`KismetMathLibrary.FClamp` (+ (* AxisValue 30.0) _returnvalue_x) -7500.0 4900.0) _returnvalue_y _returnvalue_z)))))

(event `InputAxis|MoveLeft`
  (params (AxisValue :type "Float (single-precision)"))
  (bind (_returnvalue_x _returnvalue_y _returnvalue_z) (`KismetMathLibrary.BreakVector` (`self.K2_GetActorLocation`)))
  (bind (_returnvalue_x_2 _returnvalue_y_2 _returnvalue_z_2) (`KismetMathLibrary.BreakVector` (`self.K2_GetActorLocation`)))
  ;[1 1 1] MoveRight
  (if (== AxisValue 0.0)
    (if (not (== (`self.LastMoveRightValue`) 0.0))
      (`self.K2_SetActorLocation` (`KismetMathLibrary.MakeVector` _returnvalue_x (`KismetMathLibrary.FClamp` (+ (* (`self.LastMoveRightValue`) 30.0) _returnvalue_y) -8500.0 7500.0) _returnvalue_z))
      (set `self.LastMoveRightValue` (`KismetMathLibrary.FClamp` (* (`self.LastMoveRightValue`) 0.95) -1.0)))
    (else
      (set `self.LastMoveRightValue` AxisValue)
      (`self.K2_SetActorLocation` (`KismetMathLibrary.MakeVector` _returnvalue_x_2 (`KismetMathLibrary.FClamp` (+ (* AxisValue 30.0) _returnvalue_y_2) -7500.0 7500.0) _returnvalue_z_2)))))

(event `self.ReceiveBeginPlay`
  (`self.K2_SetActorLocation` (0.0 0.0 13500.0) true true)
  (`self.K2_SetActorRotation` (struct :`Pitch` -80.0)))

(fn `UserConstructionScript`)