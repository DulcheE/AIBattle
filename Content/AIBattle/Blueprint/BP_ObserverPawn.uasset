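; Observer pawn for the AI battle: a top-down camera that pans and zooms within map bounds, with input to change game speed and cycle the game instance's display mode.
; Movement and zoom keep decaying momentum after input stops, while curves scale pan speed and set pitch by camera height.
; When the game state timer runs out, it freezes time and swaps the main HUD for the game over widget, after which Enter opens the menu map.
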(event `self.ReceiveBeginPlay`
  (bind _returnvalue (`|CreateWidget` "/Game/AIBattle/Widget/MainMap/WBP_MainWIdget.WBP_MainWIdget_C"))
  (bind _output_get (set `self.MainWidget` _returnvalue))
  (`UserWidget.AddToViewport` _output_get 0)
  (`self.K2_SetActorLocation` (0.0 0.0 13500.0) true true)
  (`self.K2_SetActorRotation` (struct :`Pitch` -80.0)))

(event `self.ReceiveTick`
  (params (DeltaSeconds :type "Float (single-precision)"))
  (bind _asgs_aibattle (cast `/Game/AIBattle/Mode/GS_AIBattle` (`GameplayStatics.GetGameState`)))
  (if (<= (`/Game/AIBattle/Mode/GS_AIBattle.GetTimer` _asgs_aibattle) 0)
    (`/Engine/EditorBlueprintResources/StandardMacros.DoOnce` false
      (:`Completed`
        (`GameplayStatics.SetGlobalTimeDilation` 0.0)
        (set `self.GameOver` true)
        (`Widget.SetVisibility` (`self.MainWidget`) "Hidden")
        (bind _returnvalue (`|CreateWidget` "/Game/AIBattle/Widget/MainMap/WBP_GameOver.WBP_GameOver_C"))
        (`UserWidget.AddToViewport` _returnvalue 0)))))

(event `InputAxis|Zoom`
  (params (AxisValue :type "Float (single-precision)"))
  (bind (_returnvalue_x _returnvalue_y _returnvalue_z) (`KismetMathLibrary.BreakVector` (`self.K2_GetActorLocation`)))
  (bind (_returnvalue_x_2 _returnvalue_y_2 _returnvalue_z_2) (`KismetMathLibrary.BreakVector` (`self.K2_GetActorLocation`)))
  (bind (_returnvalue_x_3 _returnvalue_y_3 _returnvalue_z_3) (`KismetMathLibrary.BreakVector` (`SceneComponent.K2_GetComponentLocation` (`self.Camera`))))
  ;[1 1 1] ZoomIn
  (if (== AxisValue 0.0)
    (if (not (`KismetMathLibrary.NearlyEqual_FloatFloat` (`self.LastZoomingValue`) 0.0 0.05))
      (`self.K2_SetActorLocation` (`KismetMathLibrary.MakeVector` _returnvalue_x_2 _returnvalue_y_2 (`KismetMathLibrary.FClamp` (+ (* (`self.LastZoomingValue`) 100.0) _returnvalue_z_2) 750.0 13500.0)))
      (set `self.LastZoomingValue` (`KismetMathLibrary.FClamp` (* (`self.LastZoomingValue`) 0.91) -1.0))
      (`self.K2_SetActorRotation` (`KismetMathLibrary.MakeRotator` 0.0 (+ (`CurveFloat.GetFloatValue` (`self.PitchCurve`) _returnvalue_z_3) -90.0)) :!label _label))
    (else
      (set `self.LastZoomingValue` AxisValue)
      (`self.K2_SetActorLocation` (`KismetMathLibrary.MakeVector` _returnvalue_x _returnvalue_y (`KismetMathLibrary.FClamp` (+ (* AxisValue 100.0) _returnvalue_z) 750.0 13500.0)))
      (goto _label))))

(event `InputAxis|MoveForward`
  (params (AxisValue :type "Float (single-precision)"))
  (bind (_returnvalue_x _returnvalue_y _returnvalue_z) (`KismetMathLibrary.BreakVector` (`self.K2_GetActorLocation`)))
  (bind (_returnvalue_x_2 _returnvalue_y_2 _returnvalue_z_2) (`KismetMathLibrary.BreakVector` (`self.K2_GetActorLocation`)))
  ;[1 1 1] MoveForward
  (if (== AxisValue 0.0)
    (if (not (`KismetMathLibrary.NearlyEqual_FloatFloat` (`self.LastMoveFwdValue`) 0.0 0.05))
      (`self.K2_SetActorLocation` (`KismetMathLibrary.MakeVector` (`KismetMathLibrary.FClamp` (+ (* (`self.LastMoveFwdValue`) 30.0 (`CurveFloat.GetFloatValue` (`self.CameraSpeedCurve`) _returnvalue_z_2)) _returnvalue_x_2) -7500.0 4900.0) _returnvalue_y_2 _returnvalue_z_2))
      (set `self.LastMoveFwdValue` (`KismetMathLibrary.FClamp` (* (`self.LastMoveFwdValue`) 0.95) -1.0)))
    (else
      (set `self.LastMoveFwdValue` AxisValue)
      (`self.K2_SetActorLocation` (`KismetMathLibrary.MakeVector` (`KismetMathLibrary.FClamp` (+ (* AxisValue 30.0 (`CurveFloat.GetFloatValue` (`self.CameraSpeedCurve`) _returnvalue_z)) _returnvalue_x) -7500.0 4900.0) _returnvalue_y _returnvalue_z)))))

(event `InputAxis|MoveLeft`
  (params (AxisValue :type "Float (single-precision)"))
  (bind (_returnvalue_x _returnvalue_y _returnvalue_z) (`KismetMathLibrary.BreakVector` (`self.K2_GetActorLocation`)))
  (bind (_returnvalue_x_2 _returnvalue_y_2 _returnvalue_z_2) (`KismetMathLibrary.BreakVector` (`self.K2_GetActorLocation`)))
  ;[1 1 1] MoveRight
  (if (== AxisValue 0.0)
    (if (not (`KismetMathLibrary.NearlyEqual_FloatFloat` (`self.LastMoveRightValue`) 0.0 0.05))
      (`self.K2_SetActorLocation` (`KismetMathLibrary.MakeVector` _returnvalue_x (`KismetMathLibrary.FClamp` (+ (* (`self.LastMoveRightValue`) 30.0 (`CurveFloat.GetFloatValue` (`self.CameraSpeedCurve`) _returnvalue_z)) _returnvalue_y) -8500.0 8500.0) _returnvalue_z))
      (set `self.LastMoveRightValue` (`KismetMathLibrary.FClamp` (* (`self.LastMoveRightValue`) 0.95) -1.0)))
    (else
      (set `self.LastMoveRightValue` AxisValue)
      (`self.K2_SetActorLocation` (`KismetMathLibrary.MakeVector` _returnvalue_x_2 (`KismetMathLibrary.FClamp` (+ (* AxisValue 30.0 (`CurveFloat.GetFloatValue` (`self.CameraSpeedCurve`) _returnvalue_z_2)) _returnvalue_y_2) -8500.0 8500.0) _returnvalue_z_2)))))

(event `InputAction|SlowDown`
  (params (Key :type "Key Structure"))
  (bind _currenttimedilation (`self.CurrentTimeDilation`))
  ;[1 1 1] Slow down time
  (:`Pressed`
    (if (`self.GameOver`)
      _
      (elif (<= (`self.CurrentTimeDilation`) 1.0)
        (bind _output_get (set `self.CurrentTimeDilation` (- (`KismetMathLibrary.FClamp` _currenttimedilation 0.25) 0.25)))
        (`GameplayStatics.SetGlobalTimeDilation` _output_get)
        (else
          (bind _output_get_2 (set `self.CurrentTimeDilation` (- _currenttimedilation 1.0)))
          (`GameplayStatics.SetGlobalTimeDilation` _output_get_2))))))

(event `InputAction|SpeedUp`
  (params (Key :type "Key Structure"))
  (bind _currenttimedilation (`self.CurrentTimeDilation`))
  ;[1 1 1] Speed up time
  (:`Pressed`
    (if (`self.GameOver`)
      _
      (elif (< (`self.CurrentTimeDilation`) 1.0)
        (bind _output_get (set `self.CurrentTimeDilation` (+ _currenttimedilation 0.25)))
        (`GameplayStatics.SetGlobalTimeDilation` _output_get)
        (else
          (bind _output_get_2 (set `self.CurrentTimeDilation` (+ (`KismetMathLibrary.FClamp` _currenttimedilation 1.0 4.0) 1.0)))
          (`GameplayStatics.SetGlobalTimeDilation` _output_get_2))))))

(event `Key|Enter`
  (params (Key :type "Key Structure"))
  ;[1 1 1] Enter - End Level
  (:`Pressed`
    (if (`self.GameOver`)
      (`GameplayStatics.OpenLevel` "MenuMap"))))

(event `InputAction|ChangeDisplayMode`
  (params (Key :type "Key Structure"))
  (:`Pressed`
    (bind _asgi_aibattle (cast `/Game/AIBattle/GI_AIBattle` (`GameplayStatics.GetGameInstance`)))
    (set `/Game/AIBattle/GI_AIBattle.DisplayMode` (mod (+ (`/Game/AIBattle/GI_AIBattle.DisplayMode` _asgi_aibattle) 1) 3) _asgi_aibattle)))

(fn `UserConstructionScript`)