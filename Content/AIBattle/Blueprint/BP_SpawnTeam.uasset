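; BP_SpawnTeam is a team spawn marker for the AI battle mode, showing which of two teams an area belongs to.
; The construction script uses IsTeam1 to pick the decal material, text color and default team label, so the side is visible in the editor.
; On BeginPlay it looks up that team's row in the AIBattle data table, prints the name and shows it on the text render.
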(event `self.ReceiveBeginPlay`
  (bind _returnvalue (`|GetDataTableRow` "/Game/AIBattle/AI/AIBattle.AIBattle" (select `bool` (`self.bIsTeam1`) :`false` "Team_2" :`true` "Team_1" :!type "Name"))
    (:`then`
      (bind _returnvalue_2 (`KismetTextLibrary.Conv_StringToText` (break `/Game/AIBattle/Blueprint/Struct/FTeamDescription` _returnvalue)))
      (`KismetSystemLibrary.PrintString` (`KismetTextLibrary.Conv_TextToString` _returnvalue_2))
      (`TextRenderComponent.K2_SetText` (`self.TextRender`) _returnvalue_2))))

(fn `UserConstructionScript`
  (`DecalComponent.SetDecalMaterial` (`self.Decal`) (select `bool` (`self.bIsTeam1`) :`false` "/Game/AIBattle/Material/Decals/M_TeamSpawn_Team2.M_TeamSpawn_Team2" :`true` "/Game/AIBattle/Material/Decals/M_TeamSpawn_Team1.M_TeamSpawn_Team1" :!type "MaterialInterface Object Reference"))
  (`TextRenderComponent.SetTextRenderColor` (`self.TextRender`) (select `bool` (`self.bIsTeam1`) :`false` (make `Color` 0 12 106 1) :`true` (make `Color` 128 31 4 1) :!type "Color Structure"))
  (`TextRenderComponent.K2_SetText` (`self.TextRender`) (`KismetTextLibrary.Conv_StringToText` (`KismetMathLibrary.SelectString` "Team 1" "Team 2" (`self.bIsTeam1`)))))