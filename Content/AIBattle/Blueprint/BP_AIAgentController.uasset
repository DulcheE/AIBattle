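; AI controller for BP_AIAgent pawns in an AI battle, setting team affiliation and starting the agent's behavior tree.
; After a zero-second delay on BeginPlay, it caches the agent, applies its team and runs the tree from the AIBattle data table, whose row selection is fixed to Team_2.
; AI perception updates maintain ally and enemy in-sight lists, classifying sensed agents by membership in the perceived hostile actors.
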(event `self.ReceiveBeginPlay`
  (`parent.ReceiveBeginPlay`)
  (`KismetSystemLibrary.Delay` 0.0)
  (bind _asbp_aiagent (cast `/Game/AIBattle/Blueprint/BP_AIAgent` (`self.K2_GetPawn`)))
  (bind _output_get (set `self.PossesedAgent` _asbp_aiagent))
  (bind _team (`/Game/AIBattle/Blueprint/BP_AIAgent.Team` _output_get))
  (`/Engine/EditorBlueprintResources/StandardMacros.IsValid` _team
    (:`Is Valid`
      (`self.SetTeam` (`/Game/AIBattle/Blueprint/BP_AITeam.bIsTeam1` _team))
      (bind _returnvalue (`|GetDataTableRow` "/Game/AIBattle/AI/AIBattle.AIBattle" (select `bool` false :`false` "Team_2" :`true` "Team_1" :!type "Name"))
        (:`then`
          (`self.RunBehaviorTree` (`.AI_14_E89DBE5F4F6203D0817AE28CF2FB3563` (break `/Game/AIBattle/Blueprint/Struct/FTeamDescription` _returnvalue))))))))

(event `self.AIPerception.OnTargetPerceptionUpdated`
  (params (Actor :type "Actor Object Reference") (Stimulus :type "AIStimulus Structure"))
  (bind _enemiesinsight (`self.EnemiesInSight`))
  (bind _alliesinsight (`self.AlliesInSight`))
  (bind _asbp_aiagent (cast `/Game/AIBattle/Blueprint/BP_AIAgent` Actor))
  (if (== (`KismetArrayLibrary.Array_Find` (`AIPerceptionComponent.GetPerceivedHostileActors` (`self.AIPerception`)) _asbp_aiagent) -1)
    (if Stimulus_bSuccessfullySensed
      (`KismetArrayLibrary.Array_AddUnique` _alliesinsight _asbp_aiagent)
      (else
        (`KismetArrayLibrary.Array_RemoveItem` _alliesinsight _asbp_aiagent)))
    (elif Stimulus_bSuccessfullySensed
      (`KismetArrayLibrary.Array_AddUnique` _enemiesinsight _asbp_aiagent)
      (else
        (`KismetArrayLibrary.Array_RemoveItem` _enemiesinsight _asbp_aiagent)))))

(fn `UserConstructionScript`
  (`parent.UserConstructionScript`))