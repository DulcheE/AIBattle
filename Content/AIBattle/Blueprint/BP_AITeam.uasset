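; BP_AITeam is an AI battle team actor that spawns and tracks its group of agents.
; On BeginPlay it finds the PlayerStart tagged Team1 or Team2, according to IsTeam1, and stores that transform.
; It then spawns a fixed number of BP_AIAgent actors there, adjusting for collisions.
; Each agent receives the team name, side and AgentType as its battle controller, and joins the Agents array.
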(event `self.ReceiveBeginPlay`
  (`|ExecutionSequence`
    (:`then_0`
      (bind _returnvalue (`self.GetPlayerStartTransform` (select `bool` (`self.bIsTeam1`) :`false` "Team2" :`true` "Team1" :!type "Name"))
        (:`true`
          (set `self.Spawn` _returnvalue))))
    (:`then_1`
      (for _ (range 6)
        (bind _returnvalue_2 (`|SpawnActorFromClass` "/Game/AIBattle/Blueprint/BP_AIAgent.BP_AIAgent_C" (`self.Spawn`) "AdjustIfPossibleButAlwaysSpawn" "OverrideRootScale" null (`self.Name`) (`self.bIsTeam1`) (`self.AgentType`) null))
        (`KismetArrayLibrary.Array_Add` (`self.Agents`) _returnvalue_2)))))

(fn `UserConstructionScript`)