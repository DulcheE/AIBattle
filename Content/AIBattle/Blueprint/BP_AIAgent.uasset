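; BP_AIAgent is a team-based robot agent for an AI battle, driven by AIBattleController.
; The construction script picks the body material by team, and BeginPlay hands the agent to its WBP_RobotStatus widget.
; Each tick billboards that widget toward the player's view, scaling it by a clamped square-root function of distance to stay readable.
; Getters expose clamped health and ammunition values.
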(event `self.ReceiveBeginPlay`
  (bind _aswbp_robot_status (cast `/Game/AIBattle/Widget/WBP_RobotStatus` (`WidgetComponent.GetUserWidgetObject` (`self.Widget`))))
  (set `/Game/AIBattle/Widget/WBP_RobotStatus.Agent` self _aswbp_robot_status))

(event `self.ReceiveTick`
  (params (DeltaSeconds :type "Float (single-precision)"))
  (`self.WidgetFaceCam`))

(fn `GetAmmutions`
  (returns (ReturnValue :type Integer))
  (return (`KismetMathLibrary.Clamp` (`self.Ammunitions`) 0 10)))

(fn `GetHealth`
  (returns (ReturnValue :type Integer))
  (return (`KismetMathLibrary.Clamp` (`self.Health`) 0 100)))

(fn `UserConstructionScript`
  (`PrimitiveComponent.SetMaterial` (`self.Mesh`) 1 (select `bool` (`self.bIsTeam1`) :`false` "/Game/RobotAsset/BodyMatInst2.BodyMatInst2" :`true` "/Game/RobotAsset/BodyMatInst1.BodyMatInst1" :!type "MaterialInterface Object Reference"))
  (set `self.AIControllerClass` (`self.AIBattleController`)))

(fn `WidgetFaceCam`
  (bind _returnvalue (`GameplayStatics.GetPlayerPawn` 0))
  (bind _returnvalue_2 (`SceneComponent.K2_GetComponentLocation` (`self.Widget`)))
  (bind (_outlocation _outrotation) (`self.GetActorEyesViewPoint` _returnvalue))
  (bind (_returnvalue_roll _returnvalue_pitch) (`KismetMathLibrary.BreakRotator` (`KismetMathLibrary.FindLookAtRotation` _returnvalue_2 _outlocation)))
  (`/Engine/EditorBlueprintResources/StandardMacros.IsValid` _returnvalue
    (:`Is Valid`
      (`|ExecutionSequence`
        (:`then_0`
          ;[1 1 1] Face orientation
          (`SceneComponent.K2_SetWorldRotation` (`self.Widget`) (`KismetMathLibrary.MakeRotator` 0.0 _returnvalue_pitch (.yaw _outrotation)) false false))
        (:`then_1`
          (`SceneComponent.SetRelativeScale3D` (`self.Widget`) (`KismetMathLibrary.Conv_DoubleToVector` (`KismetMathLibrary.FClamp` (- (* (`KismetMathLibrary.Sqrt` (+ (* (/ (`KismetMathLibrary.Vector_Distance` _returnvalue_2 _outlocation) 1000.0) 160.0) 320.0)) 0.5) 10.0) 1.0 10.0))))))))