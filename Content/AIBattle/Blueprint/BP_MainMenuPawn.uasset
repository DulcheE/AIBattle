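; BP_MainMenuPawn is the main menu pawn that owns and switches between the main menu and settings screens.
; On BeginPlay it creates both widgets, adds them to the viewport with settings hidden, and shows the mouse cursor.
; The CloseMainMenu and OpenMainMenu events swap widget visibility to move between the two screens without recreating them.
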(event `self.ReceiveBeginPlay`
  (bind _returnvalue (`|CreateWidget` "/Game/AIBattle/Widget/WBP_MainMenu.WBP_MainMenu_C"))
  (bind _output_get (set `self.MainMenu` _returnvalue))
  (`UserWidget.AddToViewport` _output_get 0)
  (bind _returnvalue_2 (`|CreateWidget` "/Game/AIBattle/Widget/WBP_MainMenuSettings.WBP_MainMenuSettings_C"))
  (bind _output_get_2 (set `self.Settings` _returnvalue_2))
  (`Widget.SetVisibility` _output_get_2 "Hidden")
  (`UserWidget.AddToViewport` _output_get_2 0)
  (set `PlayerController.bShowMouseCursor` true (`GameplayStatics.GetPlayerController` 0)))

(event `CloseMainMenu`
  (`Widget.SetVisibility` (`self.MainMenu`) "Hidden")
  (`Widget.SetVisibility` (`self.Settings`) "Visible"))

(event `OpenMainMenu`
  (`Widget.SetVisibility` (`self.Settings`) "Hidden")
  (`Widget.SetVisibility` (`self.MainMenu`) "Visible"))

(fn `UserConstructionScript`)