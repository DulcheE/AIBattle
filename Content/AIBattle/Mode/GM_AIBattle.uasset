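; GM_AIBattle is the game mode for an AI battle, setting up the two opposing teams when play begins.
; It reads the Team_1 and Team_2 rows from the AIBattle data table and spawns a BP_AITeam actor named from each, flagging the first as Team 1.
; Both team actors are stored on GS_AIBattle, the game state, as Team1 and Team2.
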(event `self.ReceiveBeginPlay`
  (`|ExecutionSequence`
    (:`then_0`
      ;[1 1 1] Setup teams
      (`|ExecutionSequence`
        (:`then_0`
          (bind _ref (`self.Team1Description`))
          (bind _returnvalue (`|SpawnActorFromClass` "/Game/AIBattle/Blueprint/BP_AITeam.BP_AITeam_C" (`KismetMathLibrary.MakeTransform` (0.0 0.0 0.0)) "Undefined" "OverrideRootScale" null (break `/Game/AIBattle/Blueprint/Struct/FTeamDescription` _ref) true null))
          (set `/Game/AIBattle/Mode/GS_AIBattle.Team1` _returnvalue (`self.GetGameStateAIBattle`)))
        (:`then_1`
          (bind _ref_2 (`self.Team2Description`))
          (bind _returnvalue_2 (`|SpawnActorFromClass` "/Game/AIBattle/Blueprint/BP_AITeam.BP_AITeam_C" (`KismetMathLibrary.MakeTransform` (0.0 0.0 0.0)) "Undefined" "OverrideRootScale" null (break `/Game/AIBattle/Blueprint/Struct/FTeamDescription` _ref_2) false null))
          (set `/Game/AIBattle/Mode/GS_AIBattle.Team2` _returnvalue_2 (`self.GetGameStateAIBattle`)))))))

(fn `GetGameStateAIBattle`
  (returns (ReturnValue :type "/Game/AIBattle/Mode/GS_AIBattle Object Reference"))
  (return (cast `/Game/AIBattle/Mode/GS_AIBattle` (`GameplayStatics.GetGameState`) :!pure true)))

(fn `UserConstructionScript`)