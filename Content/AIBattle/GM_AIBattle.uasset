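; GM_AIBattle is the game mode for an AI battle, setting up two competing teams when play begins.
; BeginPlay reads the Team_1 and Team_2 rows from the AIBattle data table through helper functions.
; Each row supplies the name and agent type for a spawned BP_AITeam, with the first flagged as Team 1.
; Both spawned actors are stored in the Team array in spawn order.
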(event `self.ReceiveBeginPlay`
  (`|ExecutionSequence`
    (:`then_0`
      (bind _ref (`self.Team1Description`))
      (bind _returnvalue (`|SpawnActorFromClass` "/Game/AIBattle/Blueprint/BP_AITeam.BP_AITeam_C" (`KismetMathLibrary.MakeTransform` (0.0 0.0 0.0)) "Undefined" "OverrideRootScale" null (break `/Game/AIBattle/Blueprint/Struct/FTeamDescription` _ref) (`.Agent_12_E89DBE5F4F6203D0817AE28CF2FB3563` (break `/Game/AIBattle/Blueprint/Struct/FTeamDescription` _ref)) true null))
      (`KismetArrayLibrary.Array_Add` (`self.Team`) _returnvalue))
    (:`then_1`
      (bind _ref_2 (`self.Team2Description`))
      (bind _returnvalue_2 (`|SpawnActorFromClass` "/Game/AIBattle/Blueprint/BP_AITeam.BP_AITeam_C" (`KismetMathLibrary.MakeTransform` (0.0 0.0 0.0)) "Undefined" "OverrideRootScale" null (break `/Game/AIBattle/Blueprint/Struct/FTeamDescription` _ref_2) (`.Agent_12_E89DBE5F4F6203D0817AE28CF2FB3563` (break `/Game/AIBattle/Blueprint/Struct/FTeamDescription` _ref_2)) false null))
      (`KismetArrayLibrary.Array_Add` (`self.Team`) _returnvalue_2))))

(fn `UserConstructionScript`)