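; BP_Rifle is a rifle weapon actor whose Fire event shoots toward a given target location.
; It plays the rifle fire animation and line-traces from the Muzzle socket to twice the distance of the target, ignoring itself.
; On a hit it spawns a metal impact emitter aligned to the surface normal and applies fixed damage to the hit actor.
; The trace debug drawing is left enabled.
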(event `Fire`
  (params (TargetLocation :type "Vector Structure"))
  (bind _returnvalue (`SceneComponent.GetSocketLocation` (`self.Rifle`) "Muzzle"))
  (`SkeletalMeshComponent.PlayAnimation` (`self.Rifle`) "/Game/SciFiWeapLight/Weapons/Anims/Fire_Rifle_W.Fire_Rifle_W" false)
  ;[0.6004 1 0.5714] DealDamageToEnnemi+particleEffect
  (bind (_outhit _returnvalue_2) (`KismetSystemLibrary.LineTraceSingle` _returnvalue (+ _returnvalue (* (- TargetLocation _returnvalue) 2.0)) "TraceTypeQuery3" false (`|MakeArray` self :!type "Actor Object Reference") "ForDuration" true (struct :`A` 1.0) (struct :`G` 1.0)))
  (if _returnvalue_2
    (`GameplayStatics.SpawnEmitterAtLocation` "/Game/SciFiWeapLight/FX/Particles/P_Impact_Metal_Medium_Light.P_Impact_Metal_Medium_Light" (`.Location` (`GameplayStatics.BreakHitResult` _outhit)) (`KismetMathLibrary.MakeRotFromZ` (`.Normal` (`GameplayStatics.BreakHitResult` _outhit))))
    (`GameplayStatics.ApplyDamage` (`.HitActor` (`GameplayStatics.BreakHitResult` _outhit)) 40.0)))

(fn `UserConstructionScript`)