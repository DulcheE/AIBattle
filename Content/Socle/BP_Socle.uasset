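; BP_Socle is a capture point that BP_AIAgent teams, blue or red, corrupt to take ownership.
; Sphere overlaps track agents per team, and NumberOfPlayer derives the dominant team from halved counts, flagging contested states.
; Delay loops drain the owner's corruption to neutral, then refill it for the capturing team, updating text and material.
; A looping timer heals agents while their team alone holds it; the score timer's handler is an empty stub.
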(event `self.ReceiveTick`
  (params (DeltaSeconds :type "Float (single-precision)")))

(event `self.Sphere.OnComponentBeginOverlap`
  (params (OverlappedComponent :type "PrimitiveComponent Object Reference") (OtherActor :type "Actor Object Reference") (OtherComp :type "PrimitiveComponent Object Reference") (OtherBodyIndex :type Integer) (bFromSweep :type Boolean) (SweepResult :type "HitResult Structure (by ref)"))
  (bind _asbp_aiagent (cast `/Game/AIBattle/Blueprint/BP_AIAgent` OtherActor))
  (`KismetArrayLibrary.Array_Add` (`self.PlayerOnSocle`) OtherActor)
  (if (`/Game/AIBattle/Blueprint/BP_AIAgent.bIsTeam1` _asbp_aiagent)
    (`/Engine/EditorBlueprintResources/StandardMacros.IncrementInt` (`self.NumOfBluePlayer`)
      (:`  `
        _))
    (else
      (`/Engine/EditorBlueprintResources/StandardMacros.IncrementInt` (`self.NumOfRedPlayer`)
        (:`  `
          _))))
  (`self.CheckCurentPlayer`))

(event `self.Sphere.OnComponentEndOverlap`
  (params (OverlappedComponent :type "PrimitiveComponent Object Reference") (OtherActor :type "Actor Object Reference") (OtherComp :type "PrimitiveComponent Object Reference") (OtherBodyIndex :type Integer))
  (bind _asbp_aiagent (cast `/Game/AIBattle/Blueprint/BP_AIAgent` OtherActor))
  (`KismetArrayLibrary.Array_RemoveItem` (`self.PlayerOnSocle`) OtherActor)
  (if (`/Game/AIBattle/Blueprint/BP_AIAgent.bIsTeam1` _asbp_aiagent)
    (`/Engine/EditorBlueprintResources/StandardMacros.DecrementInt` (`self.NumOfBluePlayer`)
      (:`  `
        _))
    (else
      (`/Engine/EditorBlueprintResources/StandardMacros.DecrementInt` (`self.NumOfRedPlayer`)
        (:`  `
          _))))
  (`self.CheckCurentPlayer`))

(event `CheckCurentPlayer`
  (bind (_isteam1 _numplayer) (`self.NumberOfPlayer` (`self.NumOfBluePlayer`) (`self.NumOfRedPlayer`)))
  ;[1 1 1] StartTheCorruption
  (if (== _numplayer 0)
    _
    (elif _isteam1
      (if (select `/Game/Socle/ENUM_SocleState` (`self.SocleState`) :`NewEnumerator2` true :`NewEnumerator0` true)
        (if (not (`self.Corupting?`))
          (set `self.Corupting?` true)
          (`self.ZoneCoruption` true)))
      (elif (select `/Game/Socle/ENUM_SocleState` (`self.SocleState`) :`NewEnumerator2` true :`NewEnumerator1` true)
        (if (not (`self.Corupting?`))
          (set `self.Corupting?` true)
          (`self.ZoneCoruption` false))))))

(event `ZoneCoruption`
  (params (IsTeam1 :type Boolean))
  (bind (_isteam1 _numplayer) (`self.NumberOfPlayer` (`self.NumOfBluePlayer`) (`self.NumOfRedPlayer`)))
  ;[1 1 1] UpdateCoruptionAmount
  (if (select `/Game/Socle/ENUM_SocleState` (`self.SocleState`) :`NewEnumerator2` true)
    (`PrimitiveComponent.SetMaterial` (`self.StaticMesh`) 1 "/Game/Socle/MAT_TeamNone.MAT_TeamNone")
    (if (and (== IsTeam1 _isteam1) (!= _numplayer 0))
      (if (< (`self.CorruptionAmount`) 100) :!label _label
        (if (`.OnlyOneTeam` (`self.NumberOfPlayer` (`self.NumOfBluePlayer`) (`self.NumOfRedPlayer`)))
          (bind _output_get (set `self.CorruptionAmount` (`KismetMathLibrary.Clamp` (+ (`self.CorruptionAmount`) (/ (+ (`self.NumOfBluePlayer`) (`self.NumOfRedPlayer`)) 2)) 0 100))))
        (`TextRenderComponent.K2_SetText` (`self.TextRender`) (`KismetTextLibrary.Conv_IntToText` _output_get))
        (`KismetSystemLibrary.Delay` 0.35)
        (goto _label)
        (else
          (if (`self.NumberOfPlayer` (`self.NumOfBluePlayer`) (`self.NumOfRedPlayer`))
            (set `self.SocleState` "NewEnumerator1")
            (`PrimitiveComponent.SetMaterial` (`self.StaticMesh`) 1 "/Game/Socle/MAT_TeamBlue.MAT_TeamBlue")
            (else
              (set `self.SocleState` "NewEnumerator0")
              (`PrimitiveComponent.SetMaterial` (`self.StaticMesh`) 1 "/Game/Socle/MAT_TeamRed.MAT_TeamRed")))
          (set `self.Corupting?` false))))
    (else
      (`self.RemoveOldTeam` IsTeam1))))

(event `RemoveOldTeam`
  (params (`Team1?` :type Boolean))
  (bind (_isteam1 _numplayer) (`self.NumberOfPlayer` (`self.NumOfBluePlayer`) (`self.NumOfRedPlayer`)))
  (bind _returnvalue (!= _numplayer 0))
  ;[1 1 1] RemoveOldTeam/regenearateOldTeam
  (if (> (`self.CorruptionAmount`) 0) :!label _label_2
    (if (and _returnvalue (== _isteam1 `Team1?`))
      (bind _output_get (set `self.CorruptionAmount` (`KismetMathLibrary.Clamp` (+ (`self.CorruptionAmount`) (/ (+ (`self.NumOfBluePlayer`) (`self.NumOfRedPlayer`)) -2)) 0 100)))
      (elif _returnvalue
        (bind _output_get_2 (set `self.CorruptionAmount` (`KismetMathLibrary.Clamp` (+ (`self.CorruptionAmount`) (/ (+ (`self.NumOfBluePlayer`) (`self.NumOfRedPlayer`)) 2)) 0 100)))
        (`TextRenderComponent.K2_SetText` (`self.TextRender`) (`KismetTextLibrary.Conv_IntToText` _output_get_2))
        (`KismetSystemLibrary.Delay` 0.5)
        (goto _label_2)
        (else
          _)))
    (`TextRenderComponent.K2_SetText` (`self.TextRender`) (`KismetTextLibrary.Conv_IntToText` _output_get))
    (`KismetSystemLibrary.Delay` 0.2)
    (goto _label_2)
    (else
      (set `self.SocleState` "NewEnumerator2")
      (`self.ZoneCoruption` (`self.NumberOfPlayer` (`self.NumOfBluePlayer`) (`self.NumOfRedPlayer`))))))

(event `self.ReceiveBeginPlay`
  (`KismetSystemLibrary.K2_SetTimerDelegate` (delegate `HealPlayer`) 2.0 true)
  (`KismetSystemLibrary.K2_SetTimerDelegate` (delegate `UpdateScore`) 1.0 true))

(event `UpdateScore`
  ;[1 1 1] UpdateScore
  (if (select `/Game/Socle/ENUM_SocleState` (`self.SocleState`) :`NewEnumerator1` true)
    _))

(event `HealPlayer`
  (bind (_isteam1 _numplayer _onlyoneteam) (`self.NumberOfPlayer` (`self.NumOfBluePlayer`) (`self.NumOfRedPlayer`)))
  ;[1 1 1] UpdateHealth
  (if (and _onlyoneteam (> _numplayer 0) (== _isteam1 (select `/Game/Socle/ENUM_SocleState` (`self.SocleState`) :`NewEnumerator1` true)))
    (for _index (range (+ (`KismetArrayLibrary.Array_Length` (`self.PlayerOnSocle`)) 1))
      (bind _asbp_aiagent (cast `/Game/AIBattle/Blueprint/BP_AIAgent` (`|GetArrayItem` (`self.PlayerOnSocle`) _index)))
      (`/Engine/EditorBlueprintResources/StandardMacros.IncrementInt` (`/Game/AIBattle/Blueprint/BP_AIAgent.GetHealth` _asbp_aiagent)))))

(fn `NumberOfPlayer`
  (params (NumBluePlayer :type Integer) (NumRedPlayer :type Integer))
  (returns (IsTeam1 :type Boolean) (NumPlayer :type Integer) (OnlyOneTeam :type Boolean))
  (if (== NumBluePlayer 0)
    (if (== 0 (`local.NumRedPlayer`))
      (return false 0 true)
      (else
        (return false (/ (`local.NumRedPlayer`) 2) true)))
    (elif (== 0 (`local.NumRedPlayer`))
      (return true (/ (`local.NumBluePlayer`) 2) true)
      (else
        (return false 0 false)))))

(fn `UserConstructionScript`)